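; BP_Button is a VR push button pressed by the VRpAWN's left motion controller and lit through a dynamic material's Glow parameter.
; On overlap, Tick projects controller movement onto the button's up axis, clamped to MaxTravel, and offsets the button from the controller's starting position.
; Full travel triggers glow; that or overlap end starts an interpolated return.
; ButtonInitialLoc's setter is unwired, and glow clears only upon reaching world zero.
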(event OnComponentBeginOverlap(VR_Button)
  (params (OverlappedComponent :type Primitive%20Component%20Object%20Reference) (OtherActor :type Actor%20Object%20Reference) (OtherComp :type Primitive%20Component%20Object%20Reference) (OtherBodyIndex :type Integer) (bFromSweep :type Boolean) (SweepResult :type Hit%20Result%20Structure%20%28by%20ref%29))
  (if (and (not (Variables|Default|GetbIsTracking)) (not (Variables|Default|GetbIsReturning)))
    (bind _asvrp_awn (Utilities|Casting|CastToVRpAWN OtherActor))
    (Variables|Default|SetNewVar_1 (Variables|/Game/Blueprints/VRpAWN.VRpAWN_C|GetMotionController_L _asvrp_awn))
    (Variables|Default|SetbIsTracking true)
    (Variables|Default|SetMC%20Initial%20Location (Transformation|GetWorldLocation (Variables|Default|GetNewVar_1)))))

(event OnComponentEndOverlap(VR_Button)
  (params (OverlappedComponent :type Primitive%20Component%20Object%20Reference) (OtherActor :type Actor%20Object%20Reference) (OtherComp :type Primitive%20Component%20Object%20Reference) (OtherBodyIndex :type Integer))
  (bind _asvrp_awn (Utilities|Casting|CastToVRpAWN OtherActor))
  (if (== (Variables|/Game/Blueprints/VRpAWN.VRpAWN_C|GetMotionController_L _asvrp_awn) (Variables|Default|GetNewVar_1))
    (Variables|Default|SetbIsTracking false)
    (Variables|Default|SetbIsReturning true)))

(event Custom|Fully%20Pressed
  (Rendering|Material|SetScalarParameterValue (Variables|Default|GetMI%20Button) "Glow" (Variables|Default|GetGlow%20Intensity) :!class /Script/Engine.MaterialInstanceDynamic)
  (Variables|Default|SetbIsTracking false)
  (Variables|Default|SetbIsReturning true))

(event Collision|EventActorBeginOverlap
  (params (OtherActor :type Actor%20Object%20Reference)))

(event EventTick
  (params (DeltaSeconds :type Float%20%28single-precision%29))
  (bind _vr_button (Variables|Default|GetVR_Button))
  (if (Variables|Default|GetbIsTracking)
    (Variables|Default|SetNewVar_2 (Math|Float|Clamp(Float) (Math|Float|Absolute(Float) (Math|Vector|VectorLength (Math|Vector|ProjectVectorontoVector (- (Transformation|GetWorldLocation (Variables|Default|GetNewVar_1)) (Variables|Default|GetMC%20Initial%20Location)) (Math|Vector|GetUpVector (Variables|Default|GetVR_Button))))) 0.0 (Variables|Default|GetMax%20Travel)))
    (bind _output_get (Variables|Default|SetButton%20Current%20Location (- (Variables|Default|GetMC%20Initial%20Location) (* (Math|Vector|GetUpVector _vr_button) (Variables|Default|GetNewVar_2)))))
    (Transformation|SetWorldLocation _vr_button _output_get false false)
    (if (>= (Variables|Default|GetNewVar_2) (Variables|Default|GetMax%20Travel))
      (CallFunction|FullyPressed))
    (elif (Variables|Default|GetbIsReturning)
      (bind _output_get_2 (Variables|Default|SetButton%20Current%20Location (Math|Interpolation|VInterpTo (Variables|Default|GetButton%20Current%20Location) (Variables|Default|GetButton%20Initial%20Loc) (Utilities|Time|GetWorldDeltaSeconds) (Variables|Default|GetButton%20Interp%20Speed))))
      (Transformation|SetWorldLocation (Variables|Default|GetVR_Button) _output_get_2 false false)
      (if (Class|KismetMathLibrary|EqualExactlyVectorVector (Variables|Default|GetButton%20Current%20Location) "0, 0, 0")
        (Variables|Default|SetbIsReturning false)
        (Rendering|Material|SetScalarParameterValue (Variables|Default|GetMI%20Button) "Glow" 0.0 :!class /Script/Engine.MaterialInstanceDynamic)))))

(event EventBeginPlay
  (bind _returnvalue (Rendering|Material|CreateDynamicMaterialInstance (Variables|Default|GetVR_Button) 0 "/Game/Blueprints/Button.Button" "None" :!class /Script/Engine.PrimitiveComponent))
  (Variables|Default|SetMI%20Button _returnvalue))

(fn ConstructionScript)