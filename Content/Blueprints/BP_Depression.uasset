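; BP_Depression is an interactable sphere actor that shows a pop-up widget when the player pawn enters its trigger box and hides it on exit.
; Interact turns off sphere physics, attaches to the given hand and hides the widget component; its detach branch is unreachable because the condition is fixed to true.
; While the widget is visible, Tick yaws it toward the player camera.
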(event OnComponentBeginOverlap(TriggerBox)
  (params (OverlappedComponent :type Primitive%20Component%20Object%20Reference) (OtherActor :type Actor%20Object%20Reference) (OtherComp :type Primitive%20Component%20Object%20Reference) (OtherBodyIndex :type Integer) (bFromSweep :type Boolean) (SweepResult :type Hit%20Result%20Structure%20%28by%20ref%29))
  (if (== OtherActor (Game|Player|GetPlayerPawn 0))
    (bind _aspopup_ui (Utilities|Casting|CastToPopup_UI (UserInterface|GetUserWidgetObject (Variables|Default|GetPopUpUi))))
    (Default|CallShowPopUp _aspopup_ui)))

(event OnComponentEndOverlap(TriggerBox)
  (params (OverlappedComponent :type Primitive%20Component%20Object%20Reference) (OtherActor :type Actor%20Object%20Reference) (OtherComp :type Primitive%20Component%20Object%20Reference) (OtherBodyIndex :type Integer))
  (if (== OtherActor (Game|Player|GetPlayerPawn 0))
    (bind _aspopup_ui (Utilities|Casting|CastToPopup_UI (UserInterface|GetUserWidgetObject (Variables|Default|GetPopUpUi))))
    (Default|CallHidePopUp _aspopup_ui)))

(event EventBeginPlay)

(event Collision|EventActorBeginOverlap
  (params (OtherActor :type Actor%20Object%20Reference)))

(event EventTick
  (params (DeltaSeconds :type Float%20%28single-precision%29))
  (if (Variables|/Script/Engine.SceneComponent|GetbVisible (Variables|Default|GetPopUpUi))
    (CallFunction|UpdatePopUpFacing)))

(event EventInteract
  (params (Hand :type Scene%20Component%20Object%20Reference) (bHolding :type Boolean))
  (if true
    (Physics|SetSimulatePhysics (Variables|Default|GetSphere) false)
    (Transformation|AttachComponentToComponent Hand "None" "KeepWorld" "KeepWorld" "KeepWorld" true)
    (Rendering|SetVisibility (Variables|Default|GetPopUpUi) false false)
    (else
      (Transformation|DetachFromActor "KeepWorld" "KeepWorld" "KeepWorld")
      (Physics|SetSimulatePhysics (Variables|Default|GetSphere) false)
      (Rendering|SetVisibility (Variables|Default|GetPopUpUi) true false))))

(fn ConstructionScript)

(fn UpdatePopUpFacing
  (Transformation|SetWorldRotation (Variables|Default|GetPopUpUi) (Math|Rotator|MakeRotator 0.0 0.0 (.yaw (Math|Rotator|FindLookatRotation (Transformation|GetWorldLocation (Variables|Default|GetPopUpUi)) (Camera|GetCameraLocation (Game|GetPlayerCameraManager 0))))) false false))